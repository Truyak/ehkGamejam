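; BP_Enemy is an enemy Blueprint that takes damage and reports its health to the combat UI.
; On BeginPlay it caches the player controller and its BP_HUD.
; The Damage event sends the reduced health to the HUD's CombatInterface, then stores it only while it stays above zero.
; A lethal hit has no death handling and leaves the stored Health unchanged.
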(event Custom|Damage
  (params (Amount :type Integer))
  (Default|EnemyHealthChange (Variables|/Game/_Game/Player/BP_Hud.BP_HUD_C|GetCombat%20Interface (Variables|Default|GetBP%20HUD)) (- (Variables|Default|GetHealth) Amount))
  (if (not (<= (- (Variables|Default|GetHealth) Amount) 0))
    (Variables|Default|SetHealth (- (Variables|Default|GetHealth) Amount))))

(event EventBeginPlay
  (bind _asbp_player_controller (Utilities|Casting|CastToBP_PlayerController (Game|GetPlayerController 0)))
  (bind _output_get (Variables|Default|SetBP%20Player%20Controller _asbp_player_controller))
  (bind _asbp_hud (Utilities|Casting|CastToBP_HUD (HUD|GetHUD _output_get)))
  (Variables|Default|SetBP%20HUD _asbp_hud))

(fn ConstructionScript)